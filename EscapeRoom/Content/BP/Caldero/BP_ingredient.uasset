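; BP_ingredient is an ingredient jar actor in the cauldron (Caldero) folder, coming in egg, branch and dragonfly types.
; ChangeMaterial sets the jar mesh's material from TypeOfIngredient and prints a debug letter for the type.
; Tick counts down LiveTime only while the jar simulates physics, then destroys the actor when it drops below zero.
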(event Custom|ChangeMaterial
  (bind _frasco_low (Variables|Default|Getfrasco_low))
  (if (Utilities|Enum|Equal(Enum) (Variables|Default|GetType%20of%20ingredient) "NewEnumerator0")
    (Rendering|Material|SetMaterial _frasco_low 0 "/Game/Assets_Map/Materials/Ingredientes/Antiguos/M_Ingrediente_Huevo.M_Ingrediente_Huevo")
    (Development|PrintString "H")
    (elif (Utilities|Enum|Equal(Enum) (Variables|Default|GetType%20of%20ingredient) "NewEnumerator2")
      (Rendering|Material|SetMaterial _frasco_low 0 "/Game/Assets_Map/Materials/Ingredientes/Antiguos/M_Ingrediente_Rama.M_Ingrediente_Rama")
      (Development|PrintString "R")
      (elif (Utilities|Enum|Equal(Enum) (Variables|Default|GetType%20of%20ingredient) "NewEnumerator1")
        (Rendering|Material|SetMaterial _frasco_low 0 "/Game/Assets_Map/Materials/Ingredientes/Antiguos/M_Ingrediente_Libelula.M_Ingrediente_Libelula")
        (Development|PrintString "L")))))

(event EventTick
  (params (DeltaSeconds :type Float%20%28single-precision%29))
  (if (Physics|IsSimulatingPhysics (Variables|Default|Getfrasco_low) "None")
    (Variables|Default|SetliveTime (- (Variables|Default|GetliveTime) DeltaSeconds))
    (if (< (Variables|Default|GetliveTime) 0.0)
      (Actor|DestroyActor))))

(fn ConstructionScript)