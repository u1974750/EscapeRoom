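; Cauldron-area spawner (Caldero) that creates BP_ingredient actors for the egg, dragonfly and branch items the player holds.
; Every Tick it queries the first-person character's HUD with ExistsItem, spawns at its own location, sets the ingredient type and calls ChangeMaterial.
; Only the egg's IsValid guard has its stored reference connected; the dragonfly and branch checks have empty inputs, so those spawn every frame while present.
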(event EventTick
  (params (DeltaSeconds :type Float%20%28single-precision%29))
  (bind _asbp_first_person_character (Utilities|Casting|CastToBP_FirstPersonCharacter (Game|GetPlayerCharacter 0)))
  (bind _output_get (Variables|Default|SetAs%20BP%20First%20Person%20Character _asbp_first_person_character))
  (bind _output_get_2 (Variables|Default|SetGame%20Hud%20Reference (Variables|/Game/FirstPerson/Blueprints/BP_FirstPersonCharacter.BP_FirstPersonCharacter_C|GetGameHudReference _output_get)))
  (bind _isininventory (Default|ExistsItem _output_get_2 "Ingrediente_Huevo"))
  (if _isininventory
    (Utilities|IsValid (Variables|Default|GetRefHuevo)
      (:Is%20Valid
        _)
      (:Is%20Not%20Valid
        (bind _returnvalue (Game|SpawnActorfromClass "/Game/BP/Caldero/BP_ingredient.BP_ingredient_C" (Math|Transform|MakeTransform (+ (Math|Transform|TransformLocation (Transformation|GetActorTransform) "0, 0, 0") "") "0.000000,90.000000,0.000000") "Undefined" 0 0))
        (bind _output_get_3 (Variables|Default|SetRefHuevo _returnvalue))
        (Variables|/Game/BP/Caldero/BP_ingredient.BP_ingredient_C|SetType%20of%20ingredient _output_get_3 "NewEnumerator0")
        (Default|ChangeMaterial _output_get_3)
        (Development|PrintString "Huevo"))))
  (bind _asbp_first_person_character_2 (Utilities|Casting|CastToBP_FirstPersonCharacter (Game|GetPlayerCharacter 0)))
  (bind _output_get_4 (Variables|Default|SetAs%20BP%20First%20Person%20Character _asbp_first_person_character_2))
  (bind _output_get_5 (Variables|Default|SetGame%20Hud%20Reference (Variables|/Game/FirstPerson/Blueprints/BP_FirstPersonCharacter.BP_FirstPersonCharacter_C|GetGameHudReference _output_get_4)))
  (bind _isininventory_2 (Default|ExistsItem _output_get_5 "Ingrediente_Libelula"))
  (if _isininventory_2
    (Utilities|IsValid 0
      (:Is%20Valid
        _)
      (:Is%20Not%20Valid
        (bind _returnvalue_2 (Game|SpawnActorfromClass "/Game/BP/Caldero/BP_ingredient.BP_ingredient_C" (Math|Transform|MakeTransform (+ (Math|Transform|TransformLocation (Transformation|GetActorTransform) "0, 0, 0") "") "0.000000,90.000000,0.000000") "Undefined" 0 0))
        (bind _output_get_6 (Variables|Default|SetRefLibelula _returnvalue_2))
        (Variables|/Game/BP/Caldero/BP_ingredient.BP_ingredient_C|SetType%20of%20ingredient _output_get_6 "NewEnumerator1")
        (Default|ChangeMaterial _output_get_6)
        (Development|PrintString "Libelula"))))
  (bind _asbp_first_person_character_3 (Utilities|Casting|CastToBP_FirstPersonCharacter (Game|GetPlayerCharacter 0)))
  (bind _output_get_7 (Variables|Default|SetAs%20BP%20First%20Person%20Character _asbp_first_person_character_3))
  (bind _output_get_8 (Variables|Default|SetGame%20Hud%20Reference (Variables|/Game/FirstPerson/Blueprints/BP_FirstPersonCharacter.BP_FirstPersonCharacter_C|GetGameHudReference _output_get_7)))
  (bind _isininventory_3 (Default|ExistsItem _output_get_8 "Ingrediente_Rama"))
  (if _isininventory_3
    (Utilities|IsValid 0
      (:Is%20Not%20Valid
        (bind _returnvalue_3 (Game|SpawnActorfromClass "/Game/BP/Caldero/BP_ingredient.BP_ingredient_C" (Math|Transform|MakeTransform (+ (Math|Transform|TransformLocation (Transformation|GetActorTransform) "0, 0, 0") "") "0.000000,90.000000,0.000000") "Undefined" 0 0))
        (bind _output_get_9 (Variables|Default|SetRefRama _returnvalue_3))
        (Variables|/Game/BP/Caldero/BP_ingredient.BP_ingredient_C|SetType%20of%20ingredient _output_get_9 "NewEnumerator2")
        (Default|ChangeMaterial _output_get_9)
        (Development|PrintString "Rama")))))

(fn ConstructionScript)