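; Cauldron actor that collects overlapping tagged ingredient actors, destroys them and checks their types against potion recipes.
; From three ingredients on, it concatenates enum names into an order-sensitive key for the recipe map.
; A match prints the recipe and sets a never-reset success flag; otherwise it attempts to empty the list by removing while iterating.
; Interact and StopInteract toggle the MouseGrap child actor; the I key prints ingredients for debugging.
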(event Custom|Stop%20Interact
  (bind _asmouse_grap (Utilities|Casting|CastToMouseGrap (Variables|/Script/Engine.ChildActorComponent|GetChildActor (Variables|Default|GetMouseGrap))))
  (Default|EnableToggle _asmouse_grap))

(event Custom|Interact
  (bind _asmouse_grap (Utilities|Casting|CastToMouseGrap (Variables|/Script/Engine.ChildActorComponent|GetChildActor (Variables|Default|GetMouseGrap))))
  (Default|EnableToggle _asmouse_grap))

(event EventBeginPlay)

(event Collision|EventActorBeginOverlap
  (params (OtherActor :type Actor%20Object%20Reference))
  (bind _ingredients (Variables|Default|GetIngredients))
  ;[1 1 1] Añade un el ingrediente entrado en la mezcla a la lista de ingredientes
  (if (Actor|ActorHasTag OtherActor "ingredient")
    (Development|PrintString "Ingredient add")
    (bind _asbp_ingredient (Utilities|Casting|CastToBP_ingredient OtherActor))
    (Utilities|Array|Add (Variables|Default|GetIngredients) (Variables|/Game/BP/Caldero/BP_ingredient.BP_ingredient_C|GetType%20of%20ingredient _asbp_ingredient))
    (Actor|DestroyActor OtherActor)
    ;[1 1 1] Comprueba que la receta introducida sea correcta
    (if (>= (Utilities|Array|Length (Variables|Default|GetIngredients)) 3)
      (for _array_element (Variables|Default|GetIngredients)
        (Variables|Default|SetIngredients%20Convine (Utilities|String|Append (Variables|Default|GetIngredients%20Convine) (Utilities|String|EnumtoString _array_element))))
      (bind _keys (Utilities|Map|Keys (Variables|Default|GetRecieps)))
      (for _array_element_2 _keys
        (if (Utilities|Enum|Equal(Enum) _array_element_2 (Variables|Default|GetIngredients%20Convine))
          (Variables|Default|SetPotion _array_element_2)
          (Variables|Default|SetSuccesful%20Reciep true)
          (Variables|Default|SetIngredients%20Convine "")))
      (if (Variables|Default|GetSuccesful%20Reciep)
        (Development|PrintString (.Value (Utilities|Map|Find (Variables|Default|GetRecieps) (Variables|Default|GetPotion))))
        (else
          (for _array_element_3 _ingredients
            (Utilities|Array|RemoveItem _ingredients _array_element_3)
            (Variables|Default|SetIngredients%20Convine "")))))))

(event Input|KeyboardEvents|I
  (params (Key :type Key%20Structure :default "None"))
  ;[1 1 1] Debug Lista de Ingredientes puestos
  (:Pressed
    (for _array_element (Variables|Default|GetIngredients)
      (Variables|Default|SetTextDebug (Utilities|String|Append (Variables|Default|GetTextDebug) "" (Utilities|String|EnumtoString _array_element))))
    (Development|PrintString (Variables|Default|GetTextDebug))
    (Variables|Default|SetTextDebug "")))

(fn ConstructionScript)