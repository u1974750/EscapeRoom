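; Math puzzle box that opens its lid and enables collision on the object inside when solved.
; Interact toggles cursor mode, where left-click traces find one of three dials by component name and timelines rotate it 60 degrees, tracking its position.
; Right-click looks up each dial's value and tests whether first plus third minus second equals five.
; Wrong answers trigger a Tick-driven FlipFlop shake; the original-position reset is unconnected.
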(event Custom|Interact
  (bind _returnvalue (Game|GetPlayerController 0))
  ;[1 1 1] Activa el puzzle
  (bind _output_get (Variables|Default|SetGrabMode (not (Variables|Default|GetGrabMode))))
  (if _output_get
    (Input|SetInputModeGameandUI _returnvalue 0 "DoNotLock" true false)
    (Variables|/Script/Engine.PlayerController|SetbShowMouseCursor _returnvalue true)
    (else
      (Input|SetInputModeGameOnly _returnvalue false)
      (Variables|/Script/Engine.PlayerController|SetbShowMouseCursor _returnvalue false))))

(event EventBeginPlay
  (Default|DisableCollision (Variables|Default|GetObjetoDentro))
  (Variables|Default|SetOriginalPos (.Location (Math|Transform|BreakTransform (Transformation|GetActorTransform)))))

(event EventTick
  (params (DeltaSeconds :type Float%20%28single-precision%29))
  (bind _returnvalue (Transformation|GetActorTransform))
  (bind _returnvalue_2 (Transformation|GetActorTransform))
  (bind (_location _rotation _scale) (Math|Transform|BreakTransform _returnvalue_2))
  (bind (_location_2 _rotation_2 _scale_2) (Math|Transform|BreakTransform _returnvalue))
  ;[1 1 1] Animacion Error
  (if (Variables|Default|GetdoAnimationError)
    (Utilities|FlowControl|FlipFlop
      (:A
        (Utilities|FlowControl|Delay 0.07)
        (Transformation|SetActorTransform (Math|Transform|MakeTransform (+ _location (Variables|Default|GetValuesMovError)) _rotation _scale)))
      (:B
        (Utilities|FlowControl|Delay 0.07)
        (Transformation|SetActorTransform (Math|Transform|MakeTransform (- _location_2 (Variables|Default|GetValuesMovError)) _rotation_2 _scale_2))))
    (bind _result (Math|Integer|IncrementInt (Variables|Default|GetcountN))
      (:%20%20
        (Variables|Default|SetcountN _result)
        (if (>= (Variables|Default|GetcountN) 6)
          (Variables|Default|SetdoAnimationError false)
          (Variables|Default|SetcountN 0))))))

(event Input|MouseEvents|LeftMouseButton
  (params (Key :type Key%20Structure :default "None"))
  (bind _returnvalue (Game|GetPlayerController 0))
  (bind (_worldlocation _worlddirection) (Game|Player|ConvertMouseLocationToWorldSpace _returnvalue))
  (:Pressed
    (if (Variables|Default|GetGrabMode)
      (bind (_outhit _returnvalue_2) (Collision|LineTraceByChannel _worldlocation (+ _worldlocation (* _worlddirection (Math|Float|MakeLiteralFloat 1e+05))) "TraceTypeQuery1" false 0 "None" false))
      (if _returnvalue_2
        (bind _output_get (Variables|Default|SetHitComponent (.HitComponent (Collision|BreakHitResult _outhit))))
        (if (Utilities|Enum|Equal(Enum) (Utilities|GetObjectName _output_get) "Rosca1")
          (bind _newtrack_0 (Timeline|Timeline PlayFromStart)
            (:Update
              (Transformation|SetRelativeRotation (Variables|Default|GetHitComponent) (Math|Rotator|MakeRotator 0.0 0.0 (Math|Float|Lerp (Variables|Default|GetrotationZRosca1) (+ (Variables|Default|GetrotationZRosca1) 6e+01) _newtrack_0)) false false))
            (:Finished
              (bind _output_get_2 (Variables|Default|SetrotationZRosca1 (+ (Variables|Default|GetrotationZRosca1) 6e+01)))
              (if (> _output_get_2 3e+02)
                (Variables|Default|SetrotationZRosca1 0.0)
                (Variables|Default|SetposRosca1 0.0)
                (else
                  (bind _result (Math|Float|IncrementFloat (Variables|Default|GetposRosca1))
                    (:%20%20
                      (Variables|Default|SetposRosca1 _result)))))))
          (elif (Utilities|Enum|Equal(Enum) (Utilities|GetObjectName _output_get) "Rosca2")
            (bind _newtrack_0_2 (Timeline|Timeline_0 PlayFromStart)
              (:Update
                (Transformation|SetRelativeRotation (Variables|Default|GetHitComponent) (Math|Rotator|MakeRotator 0.0 0.0 (Math|Float|Lerp (Variables|Default|GetrotationZRosca2) (+ (Variables|Default|GetrotationZRosca2) 6e+01) _newtrack_0_2)) false false))
              (:Finished
                (bind _output_get_3 (Variables|Default|SetrotationZRosca2 (+ (Variables|Default|GetrotationZRosca2) 6e+01)))
                (if (> _output_get_3 3e+02)
                  (Variables|Default|SetrotationZRosca2 0.0)
                  (Variables|Default|SetposRosca2 0.0)
                  (else
                    (bind _result_2 (Math|Float|IncrementFloat (Variables|Default|GetposRosca2))
                      (:%20%20
                        (Variables|Default|SetposRosca2 _result_2)))))))
            (elif (Utilities|Enum|Equal(Enum) (Utilities|GetObjectName _output_get) "Rosca3")
              (bind _newtrack_0_3 (Timeline|Timeline_1 PlayFromStart)
                (:Update
                  (Transformation|SetRelativeRotation (Variables|Default|GetHitComponent) (Math|Rotator|MakeRotator 0.0 0.0 (Math|Float|Lerp (Variables|Default|GetrotationZRosca3) (+ (Variables|Default|GetrotationZRosca3) 6e+01) _newtrack_0_3)) false false))
                (:Finished
                  (bind _output_get_4 (Variables|Default|SetrotationZRosca3 (+ (Variables|Default|GetrotationZRosca3) 6e+01)))
                  (if (> _output_get_4 3e+02)
                    (Variables|Default|SetrotationZRosca3 0.0)
                    (Variables|Default|SetposRosca3 0.0)
                    (else
                      (bind _result_3 (Math|Float|IncrementFloat (Variables|Default|GetposRosca3))
                        (:%20%20
                          (Variables|Default|SetposRosca3 _result_3))))))))))))))

(event Input|MouseEvents|RightMouseButton
  (params (Key :type Key%20Structure :default "None"))
  (bind _tapa (Variables|Default|GetTapa))
  (bind _returnvalue (Transformation|GetRelativeTransform _tapa))
  (bind (_location _rotation _scale) (Math|Transform|BreakTransform _returnvalue))
  ;[1 1 1] Comprueva que la solucion es correcta
  (:Pressed
    (if (Variables|Default|GetGrabMode)
      (for (_array_element _array_index) (Variables|Default|GetvaloresPosicionesRosca1)
        (if (== _array_index (Variables|Default|GetposRosca1))
          (for (_array_element_2 _array_index_2) (Variables|Default|GetvaloresPosicionesRosca2)
            (if (== _array_index_2 (Variables|Default|GetposRosca2))
              (for (_array_element_3 _array_index_3) (Variables|Default|GetvaloresPosicionesRosca3)
                (if (== _array_index_3 (Variables|Default|GetposRosca3))
                  (if (== (- (+ _array_element _array_element_3) _array_element_2) 5.0)
                    (Development|PrintString "Correcto")
                    (Variables|Default|SetComplited true)
                    ;[1 1 1] Abre la tapa y activa el contenido
                    (Transformation|SetRelativeTransform _tapa (Math|Transform|MakeTransform (Variables|/Script/Engine.SceneComponent|GetRelativeLocation (Variables|Default|GetPosTapaAbierta)) _rotation _scale) false false)
                    (Default|EnableCollision (Variables|Default|GetObjetoDentro))
                    (else
                      (Development|PrintString "Incorrecto")
                      (Variables|Default|SetdoAnimationError true))))))))))))

(fn ConstructionScript)