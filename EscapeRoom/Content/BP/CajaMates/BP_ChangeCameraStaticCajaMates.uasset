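; Trigger actor for the CajaMates puzzle that switches between the player's view and a fixed inspection camera.
; Near its box, F flip-flops the view, blocking or unblocking the player and calling Interact on the linked puzzle actor.
; Timelines move the fixed camera itself between both poses, lerping location and forward vector to fake a blend.
; Puzzle completion, polled on Tick, re-triggers the flip-flop, and the actor destroys itself after returning to the player view.
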(event OnComponentBeginOverlap(Box)
  (params (OverlappedComponent :type Primitive%20Component%20Object%20Reference) (OtherActor :type Actor%20Object%20Reference) (OtherComp :type Primitive%20Component%20Object%20Reference) (OtherBodyIndex :type Integer) (bFromSweep :type Boolean) (SweepResult :type Hit%20Result%20Structure%20%28by%20ref%29))
  ;[1 1 1] Detecta si el jugador esta cerca
  (bind _asbp_first_person_character (Utilities|Casting|CastToBP_FirstPersonCharacter OtherActor))
  (Variables|Default|SetIsPlayerNier true)
  (Default|CallErrorMessage (Variables|/Game/FirstPerson/Blueprints/BP_FirstPersonCharacter.BP_FirstPersonCharacter_C|GetErrorMessageReference _asbp_first_person_character) "F inspeccionar"))

(event OnComponentEndOverlap(Box)
  (params (OverlappedComponent :type Primitive%20Component%20Object%20Reference) (OtherActor :type Actor%20Object%20Reference) (OtherComp :type Primitive%20Component%20Object%20Reference) (OtherBodyIndex :type Integer))
  ;[1 1 1] Detecta si el jugador esta cerca
  (Utilities|Casting|CastToBP_FirstPersonCharacter OtherActor)
  (Variables|Default|SetIsPlayerNier false))

(event Custom|switchCameraFix
  (bind _returnvalue (Game|GetPlayerController 0))
  (bind _playercameramanager (Variables|/Script/Engine.PlayerController|GetPlayerCameraManager _returnvalue))
  ;[1 1 1] Cambio de camara player a camara fix
  (bind _asbp_first_person_character (Utilities|Casting|CastToBP_FirstPersonCharacter (Variables|Default|GetPlayer)))
  (Variables|/Game/FirstPerson/Blueprints/BP_FirstPersonCharacter.BP_FirstPersonCharacter_C|SetPlayerIsBlock _asbp_first_person_character true)
  (Variables|Default|SetRotCamaraPlayer (Math|Rotator|GetRotationXVector (Camera|GetCameraRotation _playercameramanager)))
  (Variables|Default|SetPosCameraPlayer (Camera|GetCameraLocation _playercameramanager))
  (Game|Player|SetViewTargetwithBlend (Game|GetPlayerController 0) (Variables|Default|GetFixCamera) 0.0 "VTBlend_Linear" 0.0 false)
  (bind _valorlerp (Timeline|Timeline PlayFromStart)
    (:Update
      (Transformation|SetActorRelativeLocation (Variables|Default|GetFixCamera) (Math|Vector|Lerp(Vector) (Variables|Default|GetPosCameraPlayer) (Variables|Default|GetPosCamaraFix) _valorlerp))
      (Transformation|SetActorRotation (Variables|Default|GetFixCamera) (Math|Conversions|RotationFromXVector (Math|Vector|Lerp(Vector) (Variables|Default|GetRotCamaraPlayer) (Variables|Default|GetRotCamaraFix) _valorlerp))))
    (:Finished
      ;[1 1 1] Indica al caldero que se inicia la interaccion
      (Default|Interact (Variables|Default|GetActor)))))

(event Custom|SwitchCameraPlayer
  ;[1 1 1] Cambio de camara fix a camara player
  (bind _asbp_first_person_character (Utilities|Casting|CastToBP_FirstPersonCharacter (Variables|Default|GetPlayer)))
  (Variables|/Game/FirstPerson/Blueprints/BP_FirstPersonCharacter.BP_FirstPersonCharacter_C|SetPlayerIsBlock _asbp_first_person_character false)
  (bind _valorlerp (Timeline|Timeline_0 PlayFromStart)
    (:Update
      (Transformation|SetActorRelativeLocation (Variables|Default|GetFixCamera) (Math|Vector|Lerp(Vector) (Variables|Default|GetPosCamaraFix) (Variables|Default|GetPosCameraPlayer) _valorlerp))
      (Transformation|SetActorRotation (Variables|Default|GetFixCamera) (Math|Conversions|RotationFromXVector (Math|Vector|Lerp(Vector) (Variables|Default|GetRotCamaraFix) (Variables|Default|GetRotCamaraPlayer) _valorlerp))))
    (:Finished
      (Game|Player|SetViewTargetwithBlend (Game|GetPlayerController 0) (Variables|Default|GetPlayer) 0.0 "VTBlend_Linear" 0.0 false)
      (if (Variables|/Game/BP/CajaMates/BP_CajaMates.BP_CajaMates_C|GetComplited (Variables|Default|GetActor))
        (Actor|DestroyActor)))))

(event Custom|PuzzleComplited
  ;[1 1 1] Flip flop entre la camara fija y la del jugador
  (if (Variables|Default|GetIsPlayerNier)
    (Utilities|FlowControl|FlipFlop
      (:A
        (CallFunction|SwitchCameraFix))
      (:B
        (Default|Interact (Variables|Default|GetActor))
        (CallFunction|SwitchCameraPlayer)))))

(event EventBeginPlay
  (bind _fixcamera (Variables|Default|GetFixCamera))
  ;[1 1 1] Guarda las posiciones de la camara fija
  (Variables|Default|SetRotCamaraFix (Math|Rotator|GetRotationXVector (Transformation|GetActorRotation _fixcamera)))
  (Variables|Default|SetPosCamaraFix (Transformation|GetActorLocation _fixcamera)))

(event EventTick
  (params (DeltaSeconds :type Float%20%28single-precision%29))
  (if (Variables|/Game/BP/CajaMates/BP_CajaMates.BP_CajaMates_C|GetComplited (Variables|Default|GetActor))
    (Utilities|FlowControl|DoOnce false
      (:Completed
        (CallFunction|PuzzleComplited)))))

(event Input|KeyboardEvents|F
  (params (Key :type Key%20Structure :default "None"))
  ;[1 1 1] Flip flop entre la camara fija y la del jugador
  (:Pressed
    (if (Variables|Default|GetIsPlayerNier)
      (Utilities|FlowControl|FlipFlop
        (:A
          (CallFunction|SwitchCameraFix))
        (:B
          (Default|Interact (Variables|Default|GetActor))
          (CallFunction|SwitchCameraPlayer))))))

(fn ConstructionScript)