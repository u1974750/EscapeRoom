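; BP_GirarModelo lets the player drag movable objects with the mouse, in a grab mode toggled by U or EnableToggle along with the cursor.
; A left-click visibility trace stores the hit component and distance.
; Tick keeps it at that distance along the cursor ray, via a PhysicsHandle for simulating bodies or SetWorldLocation otherwise.
; Releasing enables physics on the component; despite the name, nothing rotates, and the stored grab offset is unused.
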(event Custom|EnableToggle
  (bind _returnvalue (Game|GetPlayerController 0))
  (Variables|Default|SetGrabMode (not (Variables|Default|GetGrabMode)))
  (Variables|/Script/Engine.PlayerController|SetbShowMouseCursor _returnvalue (not (Variables|/Script/Engine.PlayerController|GetbShowMouseCursor _returnvalue))))

(event EventTick
  (params (DeltaSeconds :type Float%20%28single-precision%29))
  (bind _returnvalue (Game|GetPlayerController 0))
  (bind _originaldistancetoobject (Variables|Default|GetOriginalDistanceToObject))
  (bind (_worldlocation _worlddirection) (Game|Player|ConvertMouseLocationToWorldSpace _returnvalue))
  (bind _returnvalue_2 (* _worlddirection _originaldistancetoobject))
  (bind _returnvalue_3 (+ _worldlocation _returnvalue_2))
  (if (Variables|Default|GetGrabMode)
    (if (Physics|IsSimulatingPhysics (Variables|Components|GetGrabbedComponent) "None")
      (Physics|Components|PhysicsHandle|SetTargetLocation (Variables|Default|GetPhysicsHandle) _returnvalue_3)
      (else
        (Transformation|SetWorldLocation (Variables|Components|GetGrabbedComponent) _returnvalue_3 false false)))))

(event Input|KeyboardEvents|U
  (params (Key :type Key%20Structure :default "None"))
  (bind _returnvalue (Game|GetPlayerController 0))
  (:Pressed
    (Variables|Default|SetGrabMode (not (Variables|Default|GetGrabMode)))
    (Variables|/Script/Engine.PlayerController|SetbShowMouseCursor _returnvalue (not (Variables|/Script/Engine.PlayerController|GetbShowMouseCursor _returnvalue)))))

(event Input|MouseEvents|LeftMouseButton
  (params (Key :type Key%20Structure :default "None"))
  (bind _returnvalue (Game|GetPlayerController 0))
  (bind _grabmode (Variables|Default|GetGrabMode))
  (bind (_worldlocation _worlddirection) (Game|Player|ConvertMouseLocationToWorldSpace _returnvalue))
  (:Pressed
    (if _grabmode
      (bind (_outhit _returnvalue_2) (Collision|LineTraceByChannel _worldlocation (+ _worldlocation (* _worlddirection (Math|Float|MakeLiteralFloat 1e+05))) "TraceTypeQuery1" false 0 "ForDuration"))
      (if _returnvalue_2
        (if true
          (if (== (Variables|/Script/Engine.SceneComponent|GetMobility (.HitComponent (Collision|BreakHitResult _outhit))) (Math|Conversions|ToInteger(Byte) (Utilities|Enum|LiteralenumEComponentMobility "Movable")))
            (Variables|Default|SetOriginalDistanceToObject (.Distance (Collision|BreakHitResult _outhit)))
            (bind _output_get (Variables|Components|SetGrabbedComponent (.HitComponent (Collision|BreakHitResult _outhit))))
            (if (Physics|IsSimulatingPhysics _output_get "None")
              (Class|PhysicsHandleComponent|GrabComponentatLocation (Variables|Default|GetPhysicsHandle) (Variables|Components|GetGrabbedComponent) "None" (.Location (Collision|BreakHitResult _outhit)))
              (else
                (Variables|Default|SetRelativeGrabLocation (Math|Transform|InverseTransformLocation (Math|Conversions|ToTransform(Vector) (Transformation|GetWorldLocation (.HitComponent (Collision|BreakHitResult _outhit)))) (.Location (Collision|BreakHitResult _outhit)))))))))))
  (:Released
    (Physics|SetSimulatePhysics (Variables|Components|GetGrabbedComponent) true)
    (if _grabmode
      (Variables|Components|SetGrabbedComponent 0)
      (Physics|Components|PhysicsHandle|ReleaseComponent (Variables|Default|GetPhysicsHandle)))))

(fn ConstructionScript)