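; Tarot painting puzzle: the player places collected tarot cards on wall slots to remove a barricade.
; BeginPlay numbers BP_CartaPared actors by array index; Interact toggles interaction.
; Pressing T while interacting maps HUD card names to IDs, places matches and checks completion.
; Completion slides cards and barricade along Z by timeline, then destroys the actor; CartaMuerte's check is unreachable, nested under CartaMago.
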(event Custom|Interact
  ;[1 1 1] Activa y desactiva la interaccion
  (Utilities|FlowControl|FlipFlop
    (:A
      (Variables|Default|SetInteracting true))
    (:B
      (Variables|Default|SetInteracting false))))

(event Custom|CheckComplited
  ;[1 1 1] Comprueba si a sido completado
  (if (Variables|Default|GetCompletado)
    (Development|PrintString "Tarot completado")
    (bind _movetarot (Timeline|SlideTarot Play)
      (:Update
        (Transformation|AddRelativeLocation (Variables|Default|GetBP_CartaPared1) (Math|Vector|MakeVector 0.0 0.0 (Math|Float|Lerp 0.0 (Variables|Default|GetMoveTarot) _movetarot)) false false))
      (:Finished
        (Actor|DestroyActor)))))

(event Custom|GetInventoriCard
  (bind _asbp_first_person_character (Utilities|Casting|CastToBP_FirstPersonCharacter (Game|GetPlayerCharacter 0)))
  ;[0.724 0.1042 0.8698] EJEMPLO DE USO EXISTE ITEM
  (bind _cards (Default|GetTarotCards (Variables|/Game/FirstPerson/Blueprints/BP_FirstPersonCharacter.BP_FirstPersonCharacter_C|GetGameHudReference _asbp_first_person_character)))
  (if (Utilities|Array|IsEmpty _cards)
    (Development|PrintString "CARTAS VACIAS")
    (else
      (for _array_element _cards
        (if (Utilities|Enum|Equal(Enum) _array_element "cartaErmitaño")
          (Utilities|Array|Add (Variables|Default|GetCartasObtenidas) 0)
          (elif (Utilities|Enum|Equal(Enum) _array_element "CartaDiablo")
            (Utilities|Array|Add (Variables|Default|GetCartasObtenidas) 1)
            (elif (Utilities|Enum|Equal(Enum) _array_element "CartaEstrella")
              (Utilities|Array|Add (Variables|Default|GetCartasObtenidas) 2)
              (elif (Utilities|Enum|Equal(Enum) _array_element "CartaFuerza")
                (Utilities|Array|Add (Variables|Default|GetCartasObtenidas) 3)
                (elif (Utilities|Enum|Equal(Enum) _array_element "CartaSol")
                  (Utilities|Array|Add (Variables|Default|GetCartasObtenidas) 4)
                  (elif (Utilities|Enum|Equal(Enum) _array_element "CartaMago")
                    (Utilities|Array|Add (Variables|Default|GetCartasObtenidas) 5)
                    (if (Utilities|Enum|Equal(Enum) _array_element "CartaMuerte")
                      (Utilities|Array|Add (Variables|Default|GetCartasObtenidas) 6))))))))))))

(event EventBeginPlay
  ;[1 1 1] Añade los IDs a la cartas
  (bind _outactors (Actor|GetAllActorsOfClass "/Game/BP/CuadroTarot/BP_CartaPared.BP_CartaPared_C"))
  (bind _output_get (Variables|Default|SetCartasPared _outactors))
  (for (_array_element _array_index) _output_get
    (Variables|/Game/BP/CuadroTarot/BP_CartaPared.BP_CartaPared_C|SetIDCard _array_element _array_index)))

(event Input|KeyboardEvents|T
  (params (Key :type Key%20Structure :default "None"))
  ;[1 1 1] Coloca las cartas del tarot
  (:Pressed
    (if (Variables|Default|GetInteracting)
      (CallFunction|GetInventoriCard)
      (for _array_element (Variables|Default|GetCartasPared)
        (for _array_element_2 (Variables|Default|GetCartasObtenidas)
          (if (== (Variables|/Game/BP/CuadroTarot/BP_CartaPared.BP_CartaPared_C|GetIDCard _array_element) _array_element_2)
            (if (not (Utilities|Array|Get(acopy) (Variables|Default|GetCartasPuestas) _array_element_2))
              (Default|PutCard _array_element)
              (Utilities|Array|SetArrayElem (Variables|Default|GetCartasPuestas) _array_element_2 true)))))
      (Variables|Default|SetCompletado true)
      (for _array_element_3 (Variables|Default|GetCartasPuestas)
        (if (not _array_element_3)
          (Variables|Default|SetCompletado false)))
      (CallFunction|CheckComplited))))

(fn ConstructionScript)