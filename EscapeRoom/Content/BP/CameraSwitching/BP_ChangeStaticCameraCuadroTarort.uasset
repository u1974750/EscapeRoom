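; Trigger actor that toggles between the player camera and a fixed camera for an interaction, apparently the tarot painting.
; Inside its box, E flip-flops the view, blocking the player while the fixed camera is active.
; Transitions move the fixed camera itself, using Timelines to lerp location and forward vector between the player's view and its stored pose.
; ActorInteract.Interact fires once the camera arrives and again as the return begins.
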(event OnComponentBeginOverlap(Box)
  (params (OverlappedComponent :type Primitive%20Component%20Object%20Reference) (OtherActor :type Actor%20Object%20Reference) (OtherComp :type Primitive%20Component%20Object%20Reference) (OtherBodyIndex :type Integer) (bFromSweep :type Boolean) (SweepResult :type Hit%20Result%20Structure%20%28by%20ref%29))
  ;[1 1 1] Detecta si el jugador se encuentra cerca
  (Utilities|Casting|CastToBP_FirstPersonCharacter OtherActor)
  (Variables|Default|SetIsPlayerNier true))

(event OnComponentEndOverlap(Box)
  (params (OverlappedComponent :type Primitive%20Component%20Object%20Reference) (OtherActor :type Actor%20Object%20Reference) (OtherComp :type Primitive%20Component%20Object%20Reference) (OtherBodyIndex :type Integer))
  ;[1 1 1] Detecta si el jugador se encuentra cerca
  (Utilities|Casting|CastToBP_FirstPersonCharacter OtherActor)
  (Variables|Default|SetIsPlayerNier false))

(event Custom|switchCameraFix
  (bind _returnvalue (Game|GetPlayerController 0))
  (bind _playercameramanager (Variables|/Script/Engine.PlayerController|GetPlayerCameraManager _returnvalue))
  ;[1 1 1] Cambia la camar del jugador a la fija
  (bind _asbp_first_person_character (Utilities|Casting|CastToBP_FirstPersonCharacter (Variables|Default|GetPlayer)))
  (Variables|/Game/FirstPerson/Blueprints/BP_FirstPersonCharacter.BP_FirstPersonCharacter_C|SetPlayerIsBlock _asbp_first_person_character true)
  (Variables|Default|SetRotCamaraPlayer (Math|Rotator|GetRotationXVector (Camera|GetCameraRotation _playercameramanager)))
  (Variables|Default|SetPosCameraPlayer (Camera|GetCameraLocation _playercameramanager))
  (Game|Player|SetViewTargetwithBlend (Game|GetPlayerController 0) (Variables|Default|GetFixCamera) 0.0 "VTBlend_Linear" 0.0 false)
  (bind _valorlerp (Timeline|Timeline PlayFromStart)
    (:Update
      (Transformation|SetActorRelativeLocation (Variables|Default|GetFixCamera) (Math|Vector|Lerp(Vector) (Variables|Default|GetPosCameraPlayer) (Variables|Default|GetPosCamaraFix) _valorlerp))
      (Transformation|SetActorRotation (Variables|Default|GetFixCamera) (Math|Conversions|RotationFromXVector (Math|Vector|Lerp(Vector) (Variables|Default|GetRotCamaraPlayer) (Variables|Default|GetRotCamaraFix) _valorlerp))))
    (:Finished
      ;[1 1 1] Indica el inicio de la interaccion
      (Default|Interact (Variables|Default|GetActorInteract)))))

(event Custom|SwitchCameraPlayer
  ;[1 1 1] Cambia la camara fija a la del jugador
  (bind _asbp_first_person_character (Utilities|Casting|CastToBP_FirstPersonCharacter (Variables|Default|GetPlayer)))
  (Variables|/Game/FirstPerson/Blueprints/BP_FirstPersonCharacter.BP_FirstPersonCharacter_C|SetPlayerIsBlock _asbp_first_person_character false)
  (bind _valorlerp (Timeline|Timeline_0 PlayFromStart)
    (:Update
      (Transformation|SetActorRelativeLocation (Variables|Default|GetFixCamera) (Math|Vector|Lerp(Vector) (Variables|Default|GetPosCamaraFix) (Variables|Default|GetPosCameraPlayer) _valorlerp))
      (Transformation|SetActorRotation (Variables|Default|GetFixCamera) (Math|Conversions|RotationFromXVector (Math|Vector|Lerp(Vector) (Variables|Default|GetRotCamaraFix) (Variables|Default|GetRotCamaraPlayer) _valorlerp))))
    (:Finished
      (Game|Player|SetViewTargetwithBlend (Game|GetPlayerController 0) (Variables|Default|GetPlayer) 0.0 "VTBlend_Linear" 0.0 false))))

(event EventBeginPlay
  (bind _fixcamera (Variables|Default|GetFixCamera))
  ;[1 1 1] Nos guardamos la posicion y rotacion de la camara fija
  (Variables|Default|SetRotCamaraFix (Math|Rotator|GetRotationXVector (Transformation|GetActorRotation _fixcamera)))
  (Variables|Default|SetPosCamaraFix (Transformation|GetActorLocation _fixcamera)))

(event Input|KeyboardEvents|E
  (params (Key :type Key%20Structure :default "None"))
  ;[1 1 1] Flip flop entre camara fija y camara jugador
  (:Pressed
    (if (Variables|Default|GetIsPlayerNier)
      (Utilities|FlowControl|FlipFlop
        (:A
          (CallFunction|SwitchCameraFix))
        (:B
          ;[1 1 1] Le indicamos fin de la interaccion
          (Default|Interact (Variables|Default|GetActorInteract))
          (CallFunction|SwitchCameraPlayer))))))

(fn ConstructionScript)