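; Trigger actor that lets the first-person player toggle between their view and a fixed camera by pressing F inside its box.
; Switching in sets the player's block flag, makes FixCamera the view target, then timeline-lerps it from the player camera's transform to its saved one.
; Switching out clears the flag and lerps FixCamera back before returning the view target, faking a blend by moving the camera itself.
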(event OnComponentBeginOverlap(Box)
  (params (OverlappedComponent :type Primitive%20Component%20Object%20Reference) (OtherActor :type Actor%20Object%20Reference) (OtherComp :type Primitive%20Component%20Object%20Reference) (OtherBodyIndex :type Integer) (bFromSweep :type Boolean) (SweepResult :type Hit%20Result%20Structure%20%28by%20ref%29))
  (Utilities|Casting|CastToBP_FirstPersonCharacter OtherActor)
  (Variables|Default|SetIsPlayerNier true))

(event OnComponentEndOverlap(Box)
  (params (OverlappedComponent :type Primitive%20Component%20Object%20Reference) (OtherActor :type Actor%20Object%20Reference) (OtherComp :type Primitive%20Component%20Object%20Reference) (OtherBodyIndex :type Integer))
  (Utilities|Casting|CastToBP_FirstPersonCharacter OtherActor)
  (Variables|Default|SetIsPlayerNier false))

(event Custom|switchCameraFix
  (bind _returnvalue (Game|GetPlayerController 0))
  (bind _playercameramanager (Variables|/Script/Engine.PlayerController|GetPlayerCameraManager _returnvalue))
  (bind _asbp_first_person_character (Utilities|Casting|CastToBP_FirstPersonCharacter (Variables|Default|GetPlayer)))
  (Variables|/Game/FirstPerson/Blueprints/BP_FirstPersonCharacter.BP_FirstPersonCharacter_C|SetPlayerIsBlock _asbp_first_person_character true)
  (Variables|Default|SetRotCamaraPlayer (Math|Rotator|GetRotationXVector (Camera|GetCameraRotation _playercameramanager)))
  (Variables|Default|SetPosCameraPlayer (Camera|GetCameraLocation _playercameramanager))
  (Game|Player|SetViewTargetwithBlend (Game|GetPlayerController 0) (Variables|Default|GetFixCamera) 0.0 "VTBlend_Linear" 0.0 false)
  (bind _valorlerp (Timeline|Timeline PlayFromStart)
    (:Update
      (Transformation|SetActorRelativeLocation (Variables|Default|GetFixCamera) (Math|Vector|Lerp(Vector) (Variables|Default|GetPosCameraPlayer) (Variables|Default|GetPosCamaraFix) _valorlerp))
      (Transformation|SetActorRotation (Variables|Default|GetFixCamera) (Math|Conversions|RotationFromXVector (Math|Vector|Lerp(Vector) (Variables|Default|GetRotCamaraPlayer) (Variables|Default|GetRotCamaraFix) _valorlerp))))))

(event Custom|SwitchCameraPlayer
  (bind _asbp_first_person_character (Utilities|Casting|CastToBP_FirstPersonCharacter (Variables|Default|GetPlayer)))
  (Variables|/Game/FirstPerson/Blueprints/BP_FirstPersonCharacter.BP_FirstPersonCharacter_C|SetPlayerIsBlock _asbp_first_person_character false)
  (bind _valorlerp (Timeline|Timeline_0 PlayFromStart)
    (:Update
      (Transformation|SetActorRelativeLocation (Variables|Default|GetFixCamera) (Math|Vector|Lerp(Vector) (Variables|Default|GetPosCamaraFix) (Variables|Default|GetPosCameraPlayer) _valorlerp))
      (Transformation|SetActorRotation (Variables|Default|GetFixCamera) (Math|Conversions|RotationFromXVector (Math|Vector|Lerp(Vector) (Variables|Default|GetRotCamaraFix) (Variables|Default|GetRotCamaraPlayer) _valorlerp))))
    (:Finished
      (Game|Player|SetViewTargetwithBlend (Game|GetPlayerController 0) (Variables|Default|GetPlayer) 0.0 "VTBlend_Linear" 0.0 false))))

(event EventBeginPlay
  (bind _fixcamera (Variables|Default|GetFixCamera))
  (Variables|Default|SetRotCamaraFix (Math|Rotator|GetRotationXVector (Transformation|GetActorRotation _fixcamera)))
  (Variables|Default|SetPosCamaraFix (Transformation|GetActorLocation _fixcamera)))

(event Input|KeyboardEvents|F
  (params (Key :type Key%20Structure :default "None"))
  (:Pressed
    (if (Variables|Default|GetIsPlayerNier)
      (Utilities|FlowControl|FlipFlop
        (:A
          (CallFunction|SwitchCameraFix))
        (:B
          (CallFunction|SwitchCameraPlayer))))))

(fn ConstructionScript)